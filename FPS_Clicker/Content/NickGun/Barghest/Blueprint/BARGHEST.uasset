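; Barghest is a creature that runs to a preset target point and removes itself on arrival or after dying.
; BeginPlay sets the target, plays a looping animation and links the Tail and Mane meshes to the body through master pose.
; A one-second timer checks for a complete navmesh path, then issues AI MoveTo while health remains.
; At zero health, that same tick plays a one-shot animation and destroys the actor after a delay.
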(event `self.ReceiveBeginPlay`
  (set `self.Target` (`|ConvertAsset` (`self.P`)))
  ;[1 1 1] run
  (`SkinnedMeshComponent.SetLeaderPoseComponent` (`self.Tail`) (`self.Barghest`) false)
  (`SkinnedMeshComponent.SetLeaderPoseComponent` (`self.Mane`) (`self.Barghest`) false)
  (`SkeletalMeshComponent.PlayAnimation` (`self.Barghest`) null true)
  (`KismetSystemLibrary.K2_SetTimerDelegate` (delegate `Move`) 1.0 true))

(event `Move`
  (bind _returnvalue (`NavigationSystemV1.FindPathToLocationSynchronously` (`self.K2_GetActorLocation`) (`self.K2_GetActorLocation` (`self.Target`)) null null))
  (if (and (not (`NavigationPath.IsPartial` _returnvalue)) (`NavigationPath.IsValid` _returnvalue))
    (if (> (`self.B_Health`) 0)
      ;[1 1 1] go to point
      (`|AIMoveTo` self (`self.K2_GetActorLocation` (`self.Target`)) null 100.0
        (:`then`
          (if (<= (`self.B_Health`) 0) :!label _label
            ;[1 1 1] die
            (if (`self.onetime`)
              (set `self.onetime` false)
              (`SkeletalMeshComponent.PlayAnimation` (`self.Barghest`) null false)
              (`KismetSystemLibrary.Delay` 3.0)
              (`self.K2_DestroyActor`))))
        (:`OnSuccess`
          ;[1 1 1] get rid of Barghest onec gets to point
          (`self.K2_DestroyActor`)))
      (else
        (goto _label)))))

(fn `UserConstructionScript`)